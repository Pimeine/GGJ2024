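; Player character for BanaKnight, with Enhanced Input movement, look, jump and pause, plus HUD creation.
; A per-tick camera line trace sets the current target and highlights interactables.
; Interacting copies a fruit's class and mesh into a carry slot and adjusts speed; attack throws the held item, or fires a slice projectile when empty-handed.
; Gameplay tags track carrying and, with a DoOnce and falling delay, gate jumps.
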(event `self.ReceiveBeginPlay`
  (bind _returnvalue (`GameplayStatics.GetPlayerController` 0))
  (`|ExecutionSequence`
    (:`then_0`
      (bind _asplayer_controller (cast `PlayerController` (`self.GetController`)))
      (bind _returnvalue_2 (pcsubsystem `EnhancedInputLocalPlayerSubsystem` _asplayer_controller))
      (`/Engine/EditorBlueprintResources/StandardMacros.IsValid` _returnvalue_2
        (:`Is Valid`
          (`EnhancedInputSubsystemInterface.AddMappingContext` _returnvalue_2 "/Game/BanaKnight/System/IMC_Inputs.IMC_Inputs" 0 (struct)))
        (:`Is Not Valid`
          (`/Game/BanaKnight/System/Helper.H_Print` 10.0 "INVALID EIPS" self (struct :`R` 1.0 :`A` 1.0)))))
    (:`then_1`
      (`WidgetBlueprintLibrary.SetInputMode_GameOnly` _returnvalue)
      (bind _returnvalue_3 (`|CreateWidget` "/Game/BanaKnight/Widget/HUD/WBP_HUD.WBP_HUD_C" _returnvalue))
      (bind _output_get (set `self.Ref_HUD` _returnvalue_3))
      (`UserWidget.AddToViewport` _output_get 0))))

(event `E_UpdateHUDScore`
  (`/Game/BanaKnight/Widget/HUD/Components/WBPC_Score.E_UpdateScore` (`/Game/BanaKnight/Widget/HUD/WBP_HUD.WBPC_Score` (`self.Ref_HUD`))))

(event `self.ReceiveTick`
  (params (DeltaSeconds :type "Float (single-precision)"))
  (`self.F_RayChecker`) ; Check Actors Targeted by the Player
)

(event `Key|AnyKey`
  (params (Key :type "Key Structure"))
  ;[1 0 0] Any Key Checker
)

(event `EnhancedInput|/Game/BanaKnight/System/InputActions/IA_Look`
  (params (ActionValue :type "Vector2D Structure") (ElapsedSeconds :type "Float (double-precision)") (TriggeredSeconds :type "Float (double-precision)") (InputAction :type "InputAction Object Reference" :default "/Game/BanaKnight/System/InputActions/IA_Look.IA_Look"))
  ;[0 0 0] Look Around
  (:`Triggered`
    (`self.AddControllerYawInput` (* ActionValue_X -1.0))
    (`self.AddControllerPitchInput` ActionValue_Y)))

(event `EnhancedInput|/Game/BanaKnight/System/InputActions/IA_Move`
  (params (ActionValue :type "Vector2D Structure") (ElapsedSeconds :type "Float (double-precision)") (TriggeredSeconds :type "Float (double-precision)") (InputAction :type "InputAction Object Reference" :default "/Game/BanaKnight/System/InputActions/IA_Move.IA_Move"))
  (bind (_returnvalue_roll _returnvalue_pitch _returnvalue_yaw) (`KismetMathLibrary.BreakRotator` (`self.GetControlRotation`)))
  (bind (_returnvalue_roll_2 _returnvalue_pitch_2 _returnvalue_yaw_2) (`KismetMathLibrary.BreakRotator` (`self.GetControlRotation`)))
  ;[0 0 0] Move Around
  (:`Triggered`
    (`self.AddMovementInput` (`KismetMathLibrary.GetRightVector` (`KismetMathLibrary.MakeRotator` _returnvalue_roll 0.0 _returnvalue_yaw)) ActionValue_X)
    (`self.AddMovementInput` (`KismetMathLibrary.GetForwardVector` (`KismetMathLibrary.MakeRotator` 0.0 0.0 _returnvalue_yaw_2)) ActionValue_Y)))

(event `EnhancedInput|/Game/BanaKnight/System/InputActions/IA_Jump`
  (params (ActionValue :type Boolean) (ElapsedSeconds :type "Float (double-precision)") (TriggeredSeconds :type "Float (double-precision)") (InputAction :type "InputAction Object Reference" :default "/Game/BanaKnight/System/InputActions/IA_Jump.IA_Jump"))
  ;[0 0 0] Jump + Coyotee Time
  (:`Started`
    (`/Engine/EditorBlueprintResources/StandardMacros.DoOnce` false :!label _label
      (:`Completed`
        (if (`BlueprintGameplayTagLibrary.HasTag` (`self.TagContainer`) (struct :`TagName` "Status.CanJump"))
          (`self.Jump`)
          (`self.LaunchCharacter` (`KismetMathLibrary.MakeVector` 0.0 0.0 (`CharacterMovementComponent.JumpZVelocity` (`self.CharacterMovement`))))))))
  (:`Completed`
    (`self.StopJumping`)))

(event `self.K2_OnMovementModeChanged`
  (params (PrevMovementMode :type "EMovementMode Enum" :default "MOVE_None") (NewMovementMode :type "EMovementMode Enum" :default "MOVE_None") (PrevCustomMode :type Byte) (NewCustomMode :type Byte))
  ;[0 0.3695 1] Jump Fall Coyotee Check
  (if (`|EnumEquality` NewMovementMode "MOVE_Falling")
    (`BlueprintGameplayTagLibrary.RemoveGameplayTag` (`self.TagContainer`) (struct :`TagName` "Status.CanJump"))
    (`KismetSystemLibrary.RetriggerableDelay` 0.5)
    (`BlueprintGameplayTagLibrary.AddGameplayTag` (`self.TagContainer`) (struct :`TagName` "Status.CanJump"))
    (else
      (`self.E_ResetJump`))))

(event `E_ResetJump`
  ;[0 0 0] Jump + Coyotee Time
  (goto _label :!via `Reset`))

(event `EnhancedInput|/Game/BanaKnight/System/InputActions/IA_PauseGame`
  (params (ActionValue :type Boolean) (ElapsedSeconds :type "Float (double-precision)") (TriggeredSeconds :type "Float (double-precision)") (InputAction :type "InputAction Object Reference" :default "/Game/BanaKnight/System/InputActions/IA_PauseGame.IA_PauseGame"))
  ;[0 0 0] Pause Game
  (:`Started`
    (bind _returnvalue (`|CreateWidget` "/Game/BanaKnight/Widget/Menus/WBP_Pause.WBP_Pause_C"))
    (`UserWidget.AddToViewport` _returnvalue 0)))

(event `EnhancedInput|/Game/BanaKnight/System/InputActions/IA_Interact`
  (params (ActionValue :type Boolean) (ElapsedSeconds :type "Float (double-precision)") (TriggeredSeconds :type "Float (double-precision)") (InputAction :type "InputAction Object Reference" :default "/Game/BanaKnight/System/InputActions/IA_Interact.IA_Interact"))
  (bind _currenttarget (`self.CurrentTarget`))
  ;[0 0 0] Interaction
  (:`Started`
    (if (`KismetSystemLibrary.DoesImplementInterface` _currenttarget "/Game/BanaKnight/Blueprints/Interfaces/BPI_Interact.BPI_Interact_C")
      (if (not (`BlueprintGameplayTagLibrary.HasTag` (`self.TagContainer`) (struct :`TagName` "Status.Carrying")))
        (`/Engine/EditorBlueprintResources/StandardMacros.IsValid` _currenttarget
          (:`Is Valid`
            (`self.E_Interaction`)
            (message `/Game/BanaKnight/Blueprints/Interfaces/BPI_Interact.Interact` _currenttarget)))))))

(event `E_Interaction`
  (bind _carryslot (`self.CarrySlot`))
  (bind _currenttarget (`self.CurrentTarget`))
  (bind _currenttarget_2 (`self.CurrentTarget`))
  ;[1 0 0] Part to Optimize
  (`/Engine/EditorBlueprintResources/StandardMacros.IsValid` _currenttarget
    (:`Is Valid`
      (if (`KismetSystemLibrary.DoesImplementInterface` _currenttarget "/Game/BanaKnight/Blueprints/Interfaces/BPI_FruitData.BPI_FruitData_C")
        (bind (_fruitmaterial _fruitscale _fruitmesh) (message `/Game/BanaKnight/Blueprints/Interfaces/BPI_FruitData.GetFruitData` _currenttarget_2))
        (set `self.HeldItem` (`GameplayStatics.GetObjectClass` _currenttarget_2))
        (`BlueprintGameplayTagLibrary.AddGameplayTag` (`self.TagContainer`) (struct :`TagName` "Status.Carrying"))
        (`StaticMeshComponent.SetStaticMesh` _carryslot _fruitmesh)
        (`PrimitiveComponent.SetMaterial` _carryslot 0 _fruitmaterial)
        (`SceneComponent.SetWorldScale3D` _carryslot _fruitscale)
        (`self.F_UpdatePlayerSpeed` (`self.HoldingItemSpeed`))))))

(event `EnhancedInput|/Game/BanaKnight/System/InputActions/IA_Attack`
  (params (ActionValue :type Boolean) (ElapsedSeconds :type "Float (double-precision)") (TriggeredSeconds :type "Float (double-precision)") (InputAction :type "InputAction Object Reference" :default "/Game/BanaKnight/System/InputActions/IA_Attack.IA_Attack"))
  ;[1 0 0] Make the projectile start from the character's hand
  (:`Started`
    (if (`BlueprintGameplayTagLibrary.HasTag` (`self.TagContainer`) (struct :`TagName` "Status.Carrying"))
      ;[0 0 0] Throw Held Item
      (`|SpawnActorFromClass` (`self.HeldItem`) (`KismetMathLibrary.MakeTransform` (+ (`self.K2_GetActorLocation`) (* (`SceneComponent.GetForwardVector` (`self.Mesh`)) 100.0))) "Undefined" "MultiplyWithRoot" null null)
      (set `self.HeldItem` null)
      (`BlueprintGameplayTagLibrary.RemoveGameplayTag` (`self.TagContainer`) (struct :`TagName` "Status.Carrying"))
      (`StaticMeshComponent.SetStaticMesh` (`self.CarrySlot`) null)
      (`self.F_UpdatePlayerSpeed` 0.0)
      (else
        (`self.F_SpawnProjectile`)))))

(fn `F_RayChecker`
  (bind _cinecamera (`self.CineCamera`))
  (bind _returnvalue (`SceneComponent.K2_GetComponentLocation` _cinecamera))
  (bind (_outhit _returnvalue_2) (`KismetSystemLibrary.LineTraceSingle` :`Start` _returnvalue :`End` (+ _returnvalue (* (`SceneComponent.GetForwardVector` _cinecamera) 1000.0)) :`TraceChannel` "TraceTypeQuery1" :`DrawDebugType` "ForOneFrame" :`TraceColor` (struct :`G` 0.034457 :`B` 1.0 :`A` 1.0) :`DrawTime` 0.0))
  (if _returnvalue_2
    (bind (_bblockinghit _binitialoverlap _time _distance _location _impactpoint _normal _impactnormal _physmat _hitactor) (`GameplayStatics.BreakHitResult` _outhit))
    (set `self.CurrentTarget` _hitactor)
    (if (`KismetSystemLibrary.DoesImplementInterface` _hitactor "/Game/BanaKnight/Blueprints/Interfaces/BPI_Interact.BPI_Interact_C")
      (bind _output_get (set `self.PreviousTarget` (`self.CurrentTarget`)))
      (message `/Game/BanaKnight/Blueprints/Interfaces/BPI_Interact.Highlight` _output_get true)
      (else
        (bind _previoustarget (`self.PreviousTarget` :!label _label)
          (:`then`
            (message `/Game/BanaKnight/Blueprints/Interfaces/BPI_Interact.Highlight` _previoustarget false)
            (set `self.PreviousTarget` null)
            (set `self.CurrentTarget` null))
          (:`else`))))
    (else
      (goto _label))))

(fn `F_SpawnProjectile`
  (bind _returnvalue (`KismetMathLibrary.GetForwardVector` (`self.GetControlRotation`)))
  (`|SpawnActorFromClass` "/Game/BanaKnight/Blueprints/Attack/SliceProjectile/BP_SliceProjectile.BP_SliceProjectile_C" (`KismetMathLibrary.MakeTransform` (+ (+ (`self.K2_GetActorLocation`) (* _returnvalue 500.0)) (0.0 0.0 100.0)) (`KismetMathLibrary.Conv_VectorToRotator` _returnvalue)) "Undefined" "MultiplyWithRoot" null null))

(fn `F_UpdatePlayerSpeed`
  (params (SpeedAddition :type "Float (double-precision)"))
  (locals (SpeedModifier :type "Float (double-precision)"))
  (bind _charactermovement (`self.CharacterMovement`))
  (set `local.SpeedModifier` SpeedAddition)
  (set `CharacterMovementComponent.MaxWalkSpeed` (+ (`local.SpeedModifier`) (`self.NormalWalkSpeed`)) _charactermovement)
  (set `CharacterMovementComponent.JumpZVelocity` (+ (`self.NormalJumpZ`) (/ (`local.SpeedModifier`) 2.0)) _charactermovement))

(fn `getTagContainer`
  (returns (TagContainer :type "GameplayTagContainer Structure"))
  (return (`self.TagContainer`)))

(fn `UserConstructionScript`)