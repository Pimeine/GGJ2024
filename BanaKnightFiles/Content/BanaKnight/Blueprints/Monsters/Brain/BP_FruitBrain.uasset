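; BP_FruitBrain is the AI controller for fruit monsters, running the BT_Fruits behavior tree on possession.
; Its AI Perception update checks successfully sensed actors for a Player tag through the BPI_GameplayTag interface.
; A Player match clears the sight timer, while other tagged-interface actors set it with zero delay.
; The sight timer event is an empty stub, and perception writes nothing to the behavior tree.
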(event `self.ReceivePossess`
  (params (PossessedPawn :type "Pawn Object Reference"))
  (`self.RunBehaviorTree` "/Game/BanaKnight/Blueprints/Monsters/Brain/BT_Fruits.BT_Fruits"))

(event `self.AIPerception.OnTargetPerceptionUpdated`
  (params (Actor :type "Actor Object Reference") (Stimulus :type "AIStimulus Structure"))
  (if (and (`KismetSystemLibrary.DoesImplementInterface` Actor "/Game/BanaKnight/Blueprints/Interfaces/BPI_GameplayTag.BPI_GameplayTag_C") (`.bSuccessfullySensed` (break `AIStimulus` Stimulus)))
    (bind _tagcontainer (message `/Game/BanaKnight/Blueprints/Interfaces/BPI_GameplayTag.getTagContainer` Actor))
    (if (`BlueprintGameplayTagLibrary.HasTag` _tagcontainer (struct :`TagName` "Actor.Player"))
      (`KismetSystemLibrary.K2_ClearAndInvalidateTimerHandle` (`self.Timer_AI_Sight`))
      (else
        (bind _returnvalue (`KismetSystemLibrary.K2_SetTimerDelegate` (`|CreateDelegate` :!event `E_AI_Sight_Timer`)))
        (set `self.Timer_AI_Sight` _returnvalue)))))

(event `E_AI_Sight_Timer`)

(fn `UserConstructionScript`)