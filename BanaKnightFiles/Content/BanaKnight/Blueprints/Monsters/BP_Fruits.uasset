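; BP_Fruits is a fruit monster whose species ID selects a lemon or orange appearance.
; On spawn, a timeline scales it up from small to full size, and a looping timer with a randomized interval plays its voice.
; When destroyed, it plays a death sound, spawns top and bottom BP_FruitPart pieces of its species, and decrements that species' population count in GI_Banaknight.
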(event `self.ReceiveBeginPlay`
  (bind _cylinder (`self.Cylinder`))
  (`|ExecutionSequence`
    (:`then_0`
      (switch `int` (`self.Species_ActorID`)
        (:`0`
          (`StaticMeshComponent.SetStaticMesh` _cylinder "/Game/BanaKnight/Blueprints/Monsters/SM/Lemon/Lemon.Lemon"))
        (:`1`
          (`StaticMeshComponent.SetStaticMesh` _cylinder "/Game/BanaKnight/Blueprints/Monsters/SM/Orange/Orange.Orange")
          (`PrimitiveComponent.SetMaterial` _cylinder 0 "/Game/BanaKnight/Blueprints/Monsters/SM/Orange/M_Orange.M_Orange"))))
    (:`then_1`
      (`SceneComponent.SetWorldScale3D` (`self.Cylinder`) (0.2 0.2 0.2))
      (bind (_direction _growing) (`Timeline|Growing` :!via `PlayFromStart`)
        (:`Update`
          (`SceneComponent.SetWorldScale3D` (`self.Cylinder`) (`KismetMathLibrary.VLerp` (0.2 0.2 0.2) (2.0 2.0 2.0) _growing)))))
    (:`then_2`
      (`KismetSystemLibrary.K2_SetTimerDelegate` (delegate `E_Voice`) (`KismetMathLibrary.RandomFloatInRange` 2.0 4.0) true))))

(event `E_Voice`
  (`GameplayStatics.PlaySoundAtLocation` "/Game/BanaKnight/SFX/Music/WAV_FruitVoice_Cue.WAV_FruitVoice_Cue" (`self.K2_GetActorLocation`) (struct) 1.0 1.0 0.0 null null null null))

(event `self.ReceiveDestroyed`
  (bind _returnvalue (`self.GetTransform`))
  (bind _species_actorid (`self.Species_ActorID`))
  (`GameplayStatics.PlaySoundAtLocation` "/Game/BanaKnight/SFX/Music/WAV_Death_Cue.WAV_Death_Cue" (`self.K2_GetActorLocation`) (struct) 1.0 1.0 0.0 null null null null)
  (`|SpawnActorFromClass` "/Game/BanaKnight/Blueprints/Monsters/Death/BP_FruitPart.BP_FruitPart_C" _returnvalue "Undefined" "MultiplyWithRoot" null _species_actorid false null)
  (`|SpawnActorFromClass` "/Game/BanaKnight/Blueprints/Monsters/Death/BP_FruitPart.BP_FruitPart_C" _returnvalue "Undefined" "MultiplyWithRoot" null _species_actorid true null)
  (bind _asgi_banaknight (cast `/Game/BanaKnight/Blueprints/Core/GI_Banaknight` (`GameplayStatics.GetGameInstance`)))
  (switch `int` (`self.Species_ActorID`)
    (:`0`
      (bind _lemonpopulation (`/Game/BanaKnight/Blueprints/Core/GI_Banaknight.LemonPopulation` _asgi_banaknight))
      (if (> _lemonpopulation 0)
        (`/Engine/EditorBlueprintResources/StandardMacros.DecrementInt` _lemonpopulation)))
    (:`1`
      (bind _orangepopulation (`/Game/BanaKnight/Blueprints/Core/GI_Banaknight.OrangePopulation` _asgi_banaknight))
      (if (> _orangepopulation 0)
        (`/Engine/EditorBlueprintResources/StandardMacros.DecrementInt` _orangepopulation)))))

(fn `UserConstructionScript`)