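; BP_FruitPart is a fruit piece in the monster death folder, representing the top or bottom half of a lemon or orange.
; On BeginPlay it picks the static mesh and material from its species ID and Top flag.
; The construction script applies its Mass as an override on the interactable mesh and sphere collider.
; GetFruitData exposes its material, mesh, scale, mass, species and half to callers.
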(event `self.ReceiveBeginPlay`
  (bind _sm_interactableactor (`self.SM_InteractableActor`))
  (`parent.ReceiveBeginPlay`)
  (switch `int` (`self.SpieciesID`)
    (:`0`
      (if (`self.Top?`)
        (`StaticMeshComponent.SetStaticMesh` _sm_interactableactor "/Game/BanaKnight/Blueprints/Monsters/SM/Lemon/LemonPieces_Plane_004.LemonPieces_Plane_004")
        (`PrimitiveComponent.SetMaterial` _sm_interactableactor 0 "/Game/BanaKnight/Blueprints/Monsters/SM/Lemon/M_LemonTop.M_LemonTop")
        (else
          (`StaticMeshComponent.SetStaticMesh` _sm_interactableactor "/Game/BanaKnight/Blueprints/Monsters/SM/Lemon/LemonPieces_LemonBottom.LemonPieces_LemonBottom")
          (`PrimitiveComponent.SetMaterial` _sm_interactableactor 0 "/Game/BanaKnight/Blueprints/Monsters/SM/Lemon/M_LemonBottom.M_LemonBottom"))))
    (:`1`
      (if (`self.Top?`)
        (`StaticMeshComponent.SetStaticMesh` _sm_interactableactor "/Game/BanaKnight/Blueprints/Monsters/SM/Orange/OrangePieces_OrangeTop.OrangePieces_OrangeTop")
        (`PrimitiveComponent.SetMaterial` _sm_interactableactor 0 "/Game/BanaKnight/Blueprints/Monsters/SM/Orange/M_Orange_Top.M_Orange_Top")
        (else
          (`StaticMeshComponent.SetStaticMesh` _sm_interactableactor "/Game/BanaKnight/Blueprints/Monsters/SM/Orange/OrangePieces_OrangeBot.OrangePieces_OrangeBot")
          (`PrimitiveComponent.SetMaterial` _sm_interactableactor 0 "/Game/BanaKnight/Blueprints/Monsters/SM/Orange/M_Orange_Bot.M_Orange_Bot"))))))

(fn `GetFruitData`
  (returns (FruitMaterial :type "MaterialInterface Object Reference") (FruitScale :type "Vector Structure") (FruitMesh :type "StaticMesh Object Reference") (Mass :type "Float (double-precision)") (Spiecies_ID :type Integer) (`isTop?` :type Boolean))
  (bind _sm_interactableactor (`self.SM_InteractableActor`))
  (return (`PrimitiveComponent.GetMaterial` _sm_interactableactor 0) (`self.Scale`) (`StaticMeshComponent.StaticMesh` _sm_interactableactor) (`self.Mass`) (`self.SpieciesID`) (`self.Top?`)))

(fn `UserConstructionScript`
  (`parent.UserConstructionScript`)
  (`PrimitiveComponent.SetMassOverrideInKg` (`self.SM_InteractableActor`) "None" (`self.Mass`) true)
  (`PrimitiveComponent.SetMassOverrideInKg` (`self.SphereCollider`) "None" (`self.Mass`) true))