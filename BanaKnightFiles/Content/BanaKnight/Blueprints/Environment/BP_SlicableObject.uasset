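; BP_SlicableObject is an environment actor that can be sliced by projectiles.
; Its construction script copies the static mesh body into a procedural mesh with collision.
; The slice event cuts along the projectile mesh's up vector, caps the cut, and launches the new half with physics and an impulse.
; Severed halves collect in a list, with a looping timer and a clear event that destroys them as an optimization.
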(event `self.ReceiveBeginPlay`
  ;[0 0 0] Optimization Cleaner
  (`KismetSystemLibrary.K2_SetTimerDelegate` (`|CreateDelegate` :!event `E_ClearMeshesTimer`) 20.0 true))

(event `E_ClearMeshesTimer`
  ;[0 0 0] Optimization Cleaner
  (for _array_element (`self.HalfProcMeshList`)
    (`ActorComponent.K2_DestroyComponent` _array_element)))

(event `E_SliceProcMesh`
  (params (PlanePosition :type "Vector Structure") (ProjectileMesh :type "SceneComponent Object Reference"))
  (bind _outotherhalfprocmesh (`KismetProceduralMeshLibrary.SliceProceduralMesh` (`self.ProceduralMesh`) PlanePosition (`SceneComponent.GetUpVector` ProjectileMesh) true "CreateNewSectionForCap"))
  (`PrimitiveComponent.SetSimulatePhysics` _outotherhalfprocmesh true)
  (`PrimitiveComponent.AddImpulse` _outotherhalfprocmesh (500.0 500.0 500.0) "None" true)
  (`KismetArrayLibrary.Array_Add` (`self.HalfProcMeshList`) _outotherhalfprocmesh))

(fn `UserConstructionScript`
  (`KismetProceduralMeshLibrary.CopyProceduralMeshFromStaticMeshComponent` (`self.SM_ObjectBody`) 0 (`self.ProceduralMesh`) true))