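; BP_Blender is a gameplay actor in BanaKnight that scores fruit entering its blender area.
; An overlap by an actor tagged Fruit increments FruitScore on the GI_Banaknight game instance, cached at BeginPlay, then tells PC_Player to update the HUD score.
; A DoOnce reset after a short delay throttles scoring, so overlaps during that window are ignored.
; The fruit actor itself is left untouched here.
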(event `self.ReceiveBeginPlay`
  (bind _asgi_banaknight (cast `/Game/BanaKnight/Blueprints/Core/GI_Banaknight` (`GameplayStatics.GetGameInstance`)))
  (set `self.As GI Banaknight` _asgi_banaknight))

(event `self.BlenderArea.OnComponentBeginOverlap`
  (params (OverlappedComponent :type "PrimitiveComponent Object Reference") (OtherActor :type "Actor Object Reference") (OtherComp :type "PrimitiveComponent Object Reference") (OtherBodyIndex :type Integer) (bFromSweep :type Boolean) (SweepResult :type "HitResult Structure (by ref)"))
  (if (`self.ActorHasTag` OtherActor "Fruit")
    (`/Engine/EditorBlueprintResources/StandardMacros.DoOnce` false :!label _label
      (:`Completed`
        (cast `/Game/BanaKnight/Blueprints/Player/BP_Player` (`GameplayStatics.GetPlayerCharacter` 0))
        (bind _aspc_player (cast `/Game/BanaKnight/Blueprints/Core/PC_Player` (`GameplayStatics.GetPlayerController` 0)))
        (`/Engine/EditorBlueprintResources/StandardMacros.IncrementInt` (`/Game/BanaKnight/Blueprints/Core/GI_Banaknight.FruitScore` (`self.As GI Banaknight`))
          (:`  `
            (`/Game/BanaKnight/Blueprints/Core/PC_Player.E_UpdateHUDScore` _aspc_player)
            (`KismetSystemLibrary.Delay` 0.2)
            (goto _label :!via `Reset`)))))))

(fn `UserConstructionScript`)