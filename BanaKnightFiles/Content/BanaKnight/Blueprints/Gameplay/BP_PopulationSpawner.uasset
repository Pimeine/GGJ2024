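; BP_PopulationSpawner spawns BP_Fruits of one species, lemon or orange by SpieciesID, at random reachable points within its sphere radius.
; BeginPlay force-spawns four individuals and starts a looping timer.
; A checked spawn event adds fruit only while that species' GI_Banaknight population is above one and below MaxPopulation, so near-extinct species do not replenish.
; Each spawn increments that shared count.
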(event `self.ReceiveBeginPlay`
  (bind _asgi_banaknight (cast `/Game/BanaKnight/Blueprints/Core/GI_Banaknight` (`GameplayStatics.GetGameInstance`)))
  (set `self.As GI Banaknight` _asgi_banaknight)
  (`KismetSystemLibrary.K2_SetTimerDelegate` (`|CreateDelegate` :!event `E_SpawnIndividual`) 10.0 true)
  (`self.E_ForceSpawn`)
  (`self.E_ForceSpawn`)
  (`self.E_ForceSpawn`)
  (`self.E_ForceSpawn`))

(event `E_ForceSpawn`
  (`|SpawnActorFromClass` "/Game/BanaKnight/Blueprints/Monsters/BP_Fruits.BP_Fruits_C" (`KismetMathLibrary.MakeTransform` (`NavigationSystemV1.K2_GetRandomReachablePointInRadius` (`self.K2_GetActorLocation`) (`SphereComponent.SphereRadius` (`self.Sphere`)) null null) (`KismetMathLibrary.MakeRotator` 0.0 0.0 (`KismetMathLibrary.RandomFloatInRange` 0.0 360.0))) "Undefined" "MultiplyWithRoot" null (`self.Spiecies_ID`) null :!label _label)
  (`self.E_IncrementPop`))

(event `E_SpawnIndividual`
  (bind _cansummonindividual_ (`self.F_PopulationChecker`))
  (if _cansummonindividual_
    (goto _label)))

(event `E_IncrementPop`
  (bind _as_gi_banaknight (`self.As GI Banaknight`))
  (switch `int` (`self.Spiecies_ID`)
    (:`0`
      (`/Engine/EditorBlueprintResources/StandardMacros.IncrementInt` (`/Game/BanaKnight/Blueprints/Core/GI_Banaknight.LemonPopulation` _as_gi_banaknight)))
    (:`1`
      (`/Engine/EditorBlueprintResources/StandardMacros.IncrementInt` (`/Game/BanaKnight/Blueprints/Core/GI_Banaknight.OrangePopulation` _as_gi_banaknight)))))

(fn `F_PopulationChecker`
  (returns (`CanSummonIndividual?` :type Boolean))
  (locals (Loc_Pop :type Integer))
  (bind _as_gi_banaknight (`self.As GI Banaknight`))
  (switch `int` (`self.Spiecies_ID`)
    (:`0`
      (set `local.Loc_Pop` (`/Game/BanaKnight/Blueprints/Core/GI_Banaknight.LemonPopulation` _as_gi_banaknight)))
    (:`1`
      (set `local.Loc_Pop` (`/Game/BanaKnight/Blueprints/Core/GI_Banaknight.OrangePopulation` _as_gi_banaknight))))
  (if (or (>= (`local.Loc_Pop`) (`self.MaxPopulation`)) (<= (`local.Loc_Pop`) 1))
    (return false)
    (else
      (return true))))

(fn `UserConstructionScript`)